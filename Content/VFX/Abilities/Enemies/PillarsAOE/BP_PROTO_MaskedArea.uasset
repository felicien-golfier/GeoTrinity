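; Prototype enemy AOE area with a plane scaled by AreaRadius and pillar obstacles whose positions feed a material parameter collection, presumably for masking.
; The construction script scales the plane, caches the static meshes under PillarsRoot with their world locations, then writes those locations to the collection.
; Vector parameters are matched to pillars by array index rather than by name.
; BeginPlay repeats the collection write only when not on the server.
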(event EventBeginPlay
  (if (not (Networking|IsServer))
    (CallFunction|UpdateMaterialParameterCollection)))

(fn ConstructionScript
  (CallFunction|ScaleAreaSize)
  (CallFunction|SavePillarsPositions)
  (CallFunction|UpdateMaterialParameterCollection))

(fn ScaleAreaSize
  (Transformation|SetWorldScale3D (Variables|Default|GetPlane) (Math|Conversions|ToVector(Float) (Variables|Default|GetArea_Radius))))

(fn SavePillarsPositions
  (for (_array_element _array_index) (Components|GetChildrenComponents (Variables|Default|GetPillarsRoot) false)
    (bind _asstatic_mesh_component (Utilities|Casting|CastToStaticMeshComponent _array_element))
    (Utilities|Array|SetArrayElem (Variables|Default|GetObstaclesMeshes) _array_index _asstatic_mesh_component true)
    (Utilities|Array|SetArrayElem (Variables|Default|GetObstaclesLocationWS) _array_index (Transformation|GetWorldLocation _asstatic_mesh_component) true)))

(fn UpdateMaterialParameterCollection
  (bind _mpc (Variables|Default|GetMPC))
  (for (_array_element _array_index) (Variables|Default|GetObstaclesLocationWS)
    (Rendering|Material|SetVectorParameterValue _mpc (Utilities|Array|Get(acopy) (Class|MaterialParameterCollection|GetVectorParameterNames _mpc) _array_index) (Math|Conversions|ToLinearColor(Vector) _array_element) :!class /Script/Engine.KismetMaterialLibrary)))