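; Game instance Blueprint for GeoGame, intended to handle creating and joining Advanced Sessions multiplayer sessions.
; Both the create and join events are empty, as their session logic is disconnected and never runs.
; The orphaned create logic tags a session with server name and game key, then opens DraftMap as a listen server.
; The orphaned join logic joins a search result and prints success or failure.
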(event EventCreateAdvancedSession
  (params (ServerName :type String%20%28by%20ref%29) (NbOfSlots :type Integer) (bUseLan :type Boolean)))

(event EventJoinAdvancedSession
  (params (SessionData :type Blueprint%20Session%20Result%20Structure%20%28by%20ref%29)))