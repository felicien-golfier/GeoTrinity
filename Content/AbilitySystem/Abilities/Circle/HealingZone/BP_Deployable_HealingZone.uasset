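; BP_Deployable_HealingZone is the deployable healing zone of the Circle ability set, handling the zone's visual in this graph.
; BeginPlay resets the Zone component's world rotation to zero and gives it a dynamic material instance of MI_PulseCircle.
; Each Tick scales Zone to match the capsule radius and feeds GetDrainDurationRatio into the material's DurationPercent parameter.
; The graph itself contains no healing or overlap logic.
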(event EventBeginPlay
  (Transformation|SetWorldRotation (Variables|Default|GetZone) "0, 0, 0" false false)
  (bind _returnvalue (Rendering|Material|CreateDynamicMaterialInstance (Variables|Default|GetZone) 0 "/Game/Art/VFX/Generic/Materials/MI_PulseCircle.MI_PulseCircle" "ZoneMaterial" :!class /Script/Engine.PrimitiveComponent))
  (Variables|Default|SetZoneMat _returnvalue))

(event Collision|EventActorBeginOverlap
  (params (OtherActor :type Actor%20Object%20Reference)))

(event EventTick
  (params (DeltaSeconds :type Float%20%28single-precision%29))
  (Transformation|SetWorldScale3D (Variables|Default|GetZone) (Math|Conversions|ToVector(Float) (/ (Variables|/Script/Engine.CapsuleComponent|GetCapsuleRadius (Variables|Default|GetCapsuleComponent)) 5e+01)))
  (Rendering|Material|SetScalarParameterValue (Variables|Default|GetZoneMat) "DurationPercent" (Class|GeoDeployableBase|GetDrainDurationRatio) :!class /Script/Engine.MaterialInstanceDynamic))

(fn ConstructionScript)