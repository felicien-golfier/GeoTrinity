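; Enemy gameplay ability that fires projectiles in a rotating spiral over a set number of rounds, starting at a random yaw.
; On activation it commits and writes the total volley duration to the owner's Blackboard.
; LaunchProjectile loops through WaitDelay, stepping yaw evenly per shot until the count is reached, then ends the ability.
; Each delay subtracts time elapsed since the previous delay began from the shot interval, with debug timing printed.
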(event Custom|LaunchProjectile
  (bind _timeforoneround (Variables|Default|GetTimeForOneRound))
  (bind _numberprojectilebyround (Variables|Default|GetNumberProjectileByRound))
  (bind _returnvalue (/ _timeforoneround _numberprojectilebyround))
  (if (< (Variables|Default|GetIterator) (Math|Float|Truncate (* (Variables|Default|GetRoundNumber) (Variables|Default|GetNumberProjectileByRound))))
    (Variables|Default|SetIterator (+ (Variables|Default|GetIterator) 1))
    ;[0.15 0.15 0.15 0.5] Spawn projectile and wait for the next one
    (Class|GeoProjectileAbility|SpawnProjectile (Variables|Default|GetProjectileOrientation))
    (Variables|Default|SetProjectileOrientation (Math|Rotator|MakeRotator (.Roll (Math|Rotator|BreakRotator (Variables|Default|GetProjectileOrientation))) (.Pitch (Math|Rotator|BreakRotator (Variables|Default|GetProjectileOrientation))) (+ (.Yaw (Math|Rotator|BreakRotator (Variables|Default|GetProjectileOrientation))) (/ 360 (Variables|Default|GetNumberProjectileByRound)))))
    (bind _output_get (Variables|Default|SetDeltaTime (- (Utilities|Time|GetTimeSeconds) (Variables|Default|GetLastTime))))
    (Ability|Tasks|WaitDelay (- _returnvalue _output_get)
      (:then
        (Variables|Default|SetLastTime (Utilities|Time|GetTimeSeconds))
        ;[0.15 0.15 0.15 0.5] debug
        (bind _output_get_2 (Variables|Default|SetTotalTest (+ (Variables|Default|GetTotalTest) _returnvalue)))
        (Development|PrintString (Utilities|String|Append "Total test time : " (Utilities|String|ToString(Float) _output_get_2) " And  Total Time :" (Utilities|String|ToString(Float) (Class|BlackboardComponent|GetValueasFloat (AI|GetBlackboard (Ability|GetOwningActorfromActorInfo)) (Variables|Default|GetTimeKeyName))) " Iterator :" (Utilities|String|ToString(Integer) (Variables|Default|GetIterator)) " WaitTime : " (Utilities|String|ToString(Float) (- _returnvalue _output_get)) "Delta Time :" (Utilities|String|ToString(Float) (Variables|Default|GetDeltaTime))) true true "(R=0.000000,G=0.660000,B=1.000000,A=1.000000)" 0.0))
      (:OnFinish
        (CallFunction|LaunchProjectile)))
    (else
      (Ability|EndAbility))))

(event Ability|EventActivateAbility
  (bind _returnvalue (Ability|GetOwningActorfromActorInfo))
  (bind _returnvalue_2 (Transformation|GetActorRotation _returnvalue))
  (bind (_roll _pitch _yaw) (Math|Rotator|BreakRotator _returnvalue_2))
  (bind _returnvalue_3 (Ability|CommitAbility))
  (if _returnvalue_3
    (Variables|Default|SetLastTime (Utilities|Time|GetTimeSeconds))
    (AI|Components|Blackboard|SetValueasFloat (AI|GetBlackboard (Ability|GetOwningActorfromActorInfo)) (Variables|Default|GetTimeKeyName) (* (Variables|Default|GetTimeForOneRound) (Variables|Default|GetRoundNumber)))
    ;[0.15 0.15 0.15 0.5] Set First Orientation to actor forward
    (Variables|Default|SetProjectileOrientation (Math|Rotator|MakeRotator _roll _pitch (+ _yaw (Math|Random|RandomFloatinRange 0.0 3.6e+02))))
    (Variables|Default|SetIterator 0)
    (CallFunction|LaunchProjectile)
    (else
      (Ability|EndAbility))))