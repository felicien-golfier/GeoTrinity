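; Enemy ability pattern that fires projectiles in a rotating spiral over a configurable number of rounds.
; On start it offsets the payload yaw by a seed-derived angle, and the authority writes the intended total duration to the owner's Blackboard.
; LaunchProjectile then spawns one evenly stepped projectile and re-arms itself for the next tick until all are fired.
; Spawn pacing therefore follows frame rate, not the configured round time.
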(event Custom|LaunchProjectile
  (if (< (Variables|Default|GetIterator) (Math|Float|Truncate (* (Variables|Default|GetRoundNumber) (Variables|Default|GetNumberProjectileByRound))))
    (Variables|Default|SetIterator (+ (Variables|Default|GetIterator) 1))
    ;[0.15 0.15 0.15 0.5] Spawn projectile and wait for the next one
    (bind _output_get (Variables|Default|SetProjectileOrientation (+ (Variables|Default|GetProjectileOrientation) (/ 360 (Variables|Default|GetNumberProjectileByRound)))))
    (Class|ProjectilePattern|SpawnProjectile (stale EventStartPattern Payload) _output_get)
    (bind _output_get_2 (Variables|Default|SetDeltaTime (- 0.0 (Variables|Default|GetLastTime))))
    (Class|KismetSystemLibrary|SetTimerforNextTickDelegate (delegate Custom|LaunchProjectile))))

(event EventStartPattern
  (params (Payload :type Ability%20Payload%20Structure%20%28by%20ref%29))
  (bind (_origin _yaw _serverspawntime _seed _abilitylevel _abilitytag _owner _instigator) (Utilities|Struct|BreakAbilityPayload Payload))
  (Variables|Default|SetOwner _owner)
  (Variables|Default|SetInstigator _instigator)
  (Variables|Default|SetOrigin _origin)
  (Variables|Default|SetSeed _seed)
  (Variables|Default|SetYaw _yaw)
  (Variables|Default|SetLastTime 0.0)
  (if (Ability|HasAuthority (Variables|Default|GetOwner))
    (AI|Components|Blackboard|SetValueasFloat (AI|GetBlackboard (Variables|Default|GetOwner)) (Variables|Default|GetTimeKeyName) (* (Variables|Default|GetTimeForOneRound) (Variables|Default|GetRoundNumber))))
  ;[0.15 0.15 0.15 0.5] Set First Orientation to actor forward
  (Variables|Default|SetProjectileOrientation (+ (Variables|Default|GetYaw) (* (/ (Variables|Default|GetSeed) (Variables|Default|GetMaxInt32)) 360)))
  (Variables|Default|SetIterator 0)
  (CallFunction|LaunchProjectile))