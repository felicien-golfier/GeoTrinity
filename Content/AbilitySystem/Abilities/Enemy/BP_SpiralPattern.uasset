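; BP_SpiralPattern is an enemy attack pattern that fires projectiles in a rotating spiral over a set number of rounds.
; On start it writes the nominal total duration to the owner's Blackboard on authority and derives the starting angle from the payload's yaw and seed.
; LaunchProjectile steps the angle evenly and re-arms itself for the next tick, so spawning is per-frame; the configured round time only feeds the Blackboard and debug print.
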(event Custom|LaunchProjectile
  (bind _timeforoneround (Variables|Default|GetTimeForOneRound))
  (bind _numberprojectilebyround (Variables|Default|GetNumberProjectileByRound))
  (bind _returnvalue (/ _timeforoneround _numberprojectilebyround))
  (if (< (Variables|Default|GetIterator) (Math|Float|Truncate (* (Variables|Default|GetRoundNumber) (Variables|Default|GetNumberProjectileByRound))))
    (Variables|Default|SetIterator (+ (Variables|Default|GetIterator) 1))
    ;[0.15 0.15 0.15 0.5] Spawn projectile and wait for the next one
    (Variables|Default|SetProjectileOrientation (+ (Variables|Default|GetProjectileOrientation) (/ 360 (Variables|Default|GetNumberProjectileByRound))))
    (Class|Pattern|SpawnProjectile (stale EventOnStartPattern Payload) (Variables|Default|GetProjectileOrientation))
    (bind _output_get (Variables|Default|SetDeltaTime (- 0.0 (Variables|Default|GetLastTime))))
    (Class|KismetSystemLibrary|SetTimerforNextTickDelegate (delegate Custom|LaunchProjectile))
    ;[0.15 0.15 0.15 0.5] debug
    (bind _output_get_2 (Variables|Default|SetTotalTest (+ (Variables|Default|GetTotalTest) _returnvalue)))
    (Development|PrintString 0 (Utilities|String|Append "Total test time : " (Utilities|String|ToString(Float) _output_get_2) " And  Total Time :" (Utilities|String|ToString(Float) (* (Variables|Default|GetTimeForOneRound) (Variables|Default|GetRoundNumber))) " Iterator :" (Utilities|String|ToString(Integer) (Variables|Default|GetIterator)) " WaitTime : " (Utilities|String|ToString(Float) (- _returnvalue _output_get)) "Delta Time :" (Utilities|String|ToString(Float) (Variables|Default|GetDeltaTime))) true true "(R=0.000000,G=0.660000,B=1.000000,A=1.000000)" 0.0)))

(event EventOnStartPattern
  (params (Payload :type Pattern%20Payload%20Structure%20%28by%20ref%29))
  (bind (_origin _yaw _serverspawntime _seed _patternclass _owner _instigator) (Utilities|Struct|BreakPatternPayload Payload))
  (Variables|Default|SetOwner _owner)
  (Variables|Default|SetInstigator _instigator)
  (Variables|Default|SetOrigin _origin)
  (Variables|Default|SetSeed _seed)
  (Variables|Default|SetYaw _yaw)
  (Variables|Default|SetLastTime 0.0)
  (if (Ability|HasAuthority (Variables|Default|GetOwner))
    (AI|Components|Blackboard|SetValueasFloat (AI|GetBlackboard (Variables|Default|GetOwner)) (Variables|Default|GetTimeKeyName) (* (Variables|Default|GetTimeForOneRound) (Variables|Default|GetRoundNumber))))
  ;[0.15 0.15 0.15 0.5] Set First Orientation to actor forward
  (Variables|Default|SetProjectileOrientation (+ (Variables|Default|GetYaw) (* (/ (Variables|Default|GetSeed) (Variables|Default|GetMaxInt32)) 360)))
  (Variables|Default|SetIterator 0)
  (CallFunction|LaunchProjectile))