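; Passive ability component for the Square character that visualizes its gauge through pawn glow and a charge arrow.
; On BeginPlay it creates dynamic materials for the owner's mesh and an arrow actor spawned hidden at the player pawn.
; Gauge changes drive the glow, which resets on EndPlay.
; A full gauge reveals the arrow and enables Tick, which fills it over ChargeTime, then hides it and disables Tick.
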(event EventOnGaugeRatioChanged
  (params (Ratio :type Float%20%28single-precision%29))
  (bind _output_get (Variables|Default|SetLastRatio Ratio))
  (Rendering|Material|SetScalarParameterValue (Variables|Default|GetMatInst) "GlowGauge" _output_get :!class /Script/Engine.MaterialInstanceDynamic)
  (if (>= _output_get 1.0)
    (Variables|Default|SetArrowFilledValue 0.0)
    (Rendering|SetActorHiddenInGame (Variables|Default|GetArrowActor) false)
    (Components|Tick|SetComponentTickEnabled true)))

(event EventBeginPlay
  (bind _returnvalue (Game|Player|GetPlayerPawn 0))
  (bind _returnvalue_2 (Rendering|Material|CreateDynamicMaterialInstance (Actor|GetComponentbyClass (Components|GetOwner) "/Script/Engine.SkeletalMeshComponent") 0 "/Game/Characters/Meshes/Cube/MAT_PawnMat.MAT_PawnMat" "None" :!class /Script/Engine.PrimitiveComponent))
  (Variables|Default|SetMatInst _returnvalue_2)
  (bind _returnvalue_3 (Game|SpawnActorfromClass (Variables|Default|GetArrowClass) (Transformation|GetActorTransform _returnvalue) "AlwaysSpawn" "MultiplyWithRoot" 0 _returnvalue))
  (bind _output_get (Variables|Default|SetArrowActor _returnvalue_3))
  (Rendering|SetActorHiddenInGame _output_get true)
  (bind _returnvalue_4 (Rendering|Material|CreateDynamicMaterialInstance (Actor|GetComponentbyClass _output_get "/Script/Engine.StaticMeshComponent") 0 "/Game/AbilitySystem/Abilities/Square/Passive/M_ArrowfillFromTail.M_ArrowfillFromTail" "None" :!class /Script/Engine.PrimitiveComponent))
  (Variables|Default|SetArrowFillinMat _returnvalue_4))

(event EventEndPlay
  (params (EndPlayReason :type EEndPlayReason%20Enum :default "Destroyed"))
  (Rendering|Material|SetScalarParameterValue (Variables|Default|GetMatInst) "GlowGauge" 0.0 :!class /Script/Engine.MaterialInstanceDynamic))

(event EventTick
  (params (DeltaSeconds :type Float%20%28single-precision%29))
  (bind _output_get (Variables|Default|SetArrowFilledValue (+ DeltaSeconds (Variables|Default|GetArrowFilledValue))))
  (if (> (/ _output_get (Variables|Default|GetChargeTime)) 1.0)
    (Rendering|SetActorHiddenInGame (Variables|Default|GetArrowActor) true)
    (Components|Tick|SetComponentTickEnabled false)
    (else
      (Rendering|Material|SetScalarParameterValue (Variables|Default|GetArrowFillinMat) "FillAmount" (/ _output_get (Variables|Default|GetChargeTime)) :!class /Script/Engine.MaterialInstanceDynamic))))